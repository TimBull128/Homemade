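; Inventory component that stores Enemy, Weapon and Tool actors in separate indexed lists, plus a money total.
; AddNew marks an item non-pickupable and holds it; UpdateActorHeld steps the active category's index via NewIDX.
; SetActorHeld hides the previous item and attaches the new one to the owning Character's InventorySocket, setting collision by type.
; DetachActorHeld drops by spawning a same-class replacement, copying details through interface messages, and destroying the original.
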(fn `Add Money`
  (params (`Add Money` :type Integer))
  (set `self.Money` (+ `Add Money` (`self.Money`))))

(fn `Add New`
  (params (`New Actor` :type "Actor Object Reference"))
  (locals (`Target actor` :type "Actor Object Reference"))
  (bind _enemies (`self.Enemies`))
  (bind _tools (`self.Tools`))
  (bind _weapons (`self.Weapons`))
  (`/Engine/EditorBlueprintResources/StandardMacros.IsValid` `New Actor`
    (:`Is Valid`
      (bind _output_get (set `local.Target actor` `New Actor`))
      (bind _actor_details (message `/Game/Blueprints/Functions/BPI_Interact.Get Actor Details` _output_get))
      (bind _structout (setmembers `/Game/Blueprints/Functions/S_ActorDetails` :`StructRef` _actor_details :`isPickupable?` false))
      (message `/Game/Blueprints/Functions/BPI_Interact.Set Actor Details` _output_get _structout)
      (bind _output_get_2 (set `self.Inventory Type` (`.InventoryType_20_7964C2304E97BEB78DCB259AD7C0D2BE` (break `/Game/Blueprints/Functions/S_ActorDetails` _structout))))
      (switch `/Game/Blueprints/Functions/E_InventoryType` _output_get_2
        (:`NewEnumerator0`
          (bind _returnvalue (`KismetArrayLibrary.Array_AddUnique` (`.Actors_5_8C4CCAFF425DF7AD96388EBCA6A19ADB` (break `/Game/Blueprints/Functions/S_InventoryAssets` _enemies)) (`local.Target actor`)))
          (bind _structout_2 (setmembers `/Game/Blueprints/Functions/S_InventoryAssets` :`StructRef` _enemies :`Index` _returnvalue))
          (`self.Set Actor Held` _structout_2)
          (return))
        (:`NewEnumerator4`
          (bind _returnvalue_2 (`KismetArrayLibrary.Array_AddUnique` (`.Actors_5_8C4CCAFF425DF7AD96388EBCA6A19ADB` (break `/Game/Blueprints/Functions/S_InventoryAssets` _weapons)) (`local.Target actor`)))
          (bind _structout_3 (setmembers `/Game/Blueprints/Functions/S_InventoryAssets` :`StructRef` _weapons :`Index` _returnvalue_2))
          (`self.Set Actor Held` _structout_3)
          (return))
        (:`NewEnumerator5`
          (bind _returnvalue_3 (`KismetArrayLibrary.Array_AddUnique` (`.Actors_5_8C4CCAFF425DF7AD96388EBCA6A19ADB` (break `/Game/Blueprints/Functions/S_InventoryAssets` _tools)) (`local.Target actor`)))
          (bind _structout_4 (setmembers `/Game/Blueprints/Functions/S_InventoryAssets` :`StructRef` _tools :`Index` _returnvalue_3))
          (`self.Set Actor Held` _structout_4)
          (return))))))

(fn `Detach Actor Held`
  (params (SpawnTransform :type "Transform Structure"))
  (returns (ReturnValue :type "Actor Object Reference"))
  (bind _actor_held (`self.Actor Held`))
  (`Actor.K2_DetachFromActor` _actor_held "KeepWorld" "KeepWorld" "KeepWorld")
  (bind _returnvalue (`|SpawnActorFromClass` (`GameplayStatics.GetObjectClass` _actor_held) SpawnTransform "Undefined" "MultiplyWithRoot" null null))
  (switch `/Game/Blueprints/Functions/E_InventoryType` (`self.Inventory Type`)
    (:`NewEnumerator0`
      (`KismetArrayLibrary.Array_RemoveItem` (`.Actors_5_8C4CCAFF425DF7AD96388EBCA6A19ADB` (break `/Game/Blueprints/Functions/S_InventoryAssets` (`self.Enemies`)))))
    (:`NewEnumerator4`
      (`KismetArrayLibrary.Array_RemoveItem` (`.Actors_5_8C4CCAFF425DF7AD96388EBCA6A19ADB` (break `/Game/Blueprints/Functions/S_InventoryAssets` (`self.Weapons`)))))
    (:`NewEnumerator5`
      (`KismetArrayLibrary.Array_RemoveItem` (`.Actors_5_8C4CCAFF425DF7AD96388EBCA6A19ADB` (break `/Game/Blueprints/Functions/S_InventoryAssets` (`self.Tools`))))))
  (bind _actor_details (message `/Game/Blueprints/Functions/BPI_Interact.Get Actor Details` _actor_held))
  (message `/Game/Blueprints/Functions/BPI_Interact.Set Actor Details` _returnvalue _actor_details)
  (`Actor.K2_DestroyActor` _actor_held)
  (`self.Update Actor Held` 0)
  (return _returnvalue))

(fn `New IDX`
  (params (InputPin :type Integer) (S_InventoryAssets :type "/Game/Blueprints/Functions/S_InventoryAssets Structure (by ref)"))
  (returns (ReturnValue :type Integer))
  (locals (ArrLen :type Integer :default 0)))

(fn `Set Actor Held`
  (params (Inventory :type "/Game/Blueprints/Functions/S_InventoryAssets Structure"))
  (returns (OutputPin :type "Actor Object Reference"))
  (bind _actor_held (`self.Actor Held`))
  (if (== Inventory_Index_7_7851C67547B7B657D7148DA25AA02D3A -1)
    (return null)
    (else
      (bind _actor_held_2 (`self.Actor Held`)
        (:`then`
          (`Actor.K2_DetachFromActor` _actor_held_2 "KeepWorld" "KeepWorld" "KeepWorld")
          (`Actor.SetActorHiddenInGame` _actor_held_2 true)
          (message `/Game/Blueprints/Functions/BPI_Interact.Set Object Collision` _actor_held_2 "NoCollision"))
        (:`else`
          _))
      (bind _output_get (set `self.Actor Held` (`|GetArrayItem` Inventory_Actors_5_8C4CCAFF425DF7AD96388EBCA6A19ADB Inventory_Index_7_7851C67547B7B657D7148DA25AA02D3A)))
      (`/Engine/EditorBlueprintResources/StandardMacros.IsValid` _output_get
        (:`Is Valid`
          (bind _ascharacter (cast `Character` (`self.GetOwner`)))
          (`Actor.SetActorHiddenInGame` _output_get false)
          (bind _actor_details (message `/Game/Blueprints/Functions/BPI_Interact.Get Actor Details` _output_get))
          (switch `/Game/Blueprints/Functions/E_InventoryType` (`.InventoryType_20_7964C2304E97BEB78DCB259AD7C0D2BE` (break `/Game/Blueprints/Functions/S_ActorDetails` _actor_details))
            (:`NewEnumerator0`
              (`Actor.SetActorEnableCollision` _actor_held false :!label _label))
            (:`NewEnumerator4`
              (message `/Game/Blueprints/Functions/BPI_Interact.Set Object Collision` _actor_held "QueryOnly"))
            (:`NewEnumerator5`
              (goto _label)))
          (`Actor.K2_AttachToComponent` _actor_held (`Character.Mesh` _ascharacter) "InventorySocket" "SnapToTarget" "SnapToTarget" "KeepWorld" false)
          (return (`self.Actor Held`)))
        (:`Is Not Valid`
          (return null))))))

(fn `Update Actor Held`
  (params (`Index Update` :type Integer))
  (locals (`Update IDX` :type Integer))
  (set `local.Update IDX` `Index Update`)
  (switch `/Game/Blueprints/Functions/E_InventoryType` (`self.Inventory Type`)
    (:`NewEnumerator0`
      (bind _returnvalue (`self.New IDX` (`local.Update IDX`) (`self.Enemies`)))
      (bind _structout (setmembers `/Game/Blueprints/Functions/S_InventoryAssets` :`StructRef` (`self.Enemies`) :`Index` _returnvalue))
      (`self.Set Actor Held` _structout))
    (:`NewEnumerator4`
      (bind _returnvalue_2 (`self.New IDX` (`local.Update IDX`) (`self.Weapons`)))
      (bind _structout_2 (setmembers `/Game/Blueprints/Functions/S_InventoryAssets` :`StructRef` (`self.Weapons`) :`Index` _returnvalue_2))
      (`self.Set Actor Held` _structout_2))
    (:`NewEnumerator5`
      (bind _returnvalue_3 (`self.New IDX` (`local.Update IDX`) (`self.Tools`)))
      (bind _structout_3 (setmembers `/Game/Blueprints/Functions/S_InventoryAssets` :`StructRef` (`self.Tools`) :`Index` _returnvalue_3))
      (`self.Set Actor Held` _structout_3))))