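; Health component that tracks an actor's current health and alive or dead status.
; Initialization fills health to maximum, and damage is only applied while alive, clamped, printed to screen and broadcast through OnHealthChanged.
; The component listens to its own dispatchers: zero health fires OnDeath, which flips the status enum so further damage is ignored.
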(event `self.ReceiveBeginPlay`
  (add `self.OnDeath` (delegate `OnDeath_Event`))
  (add `self.OnHealthChanged` (delegate `OnHealthChanged_Event`)))

(event `OnDeath_Event`
  (`self.Die`))

(event `OnHealthChanged_Event`
  (if (== (`self.Current Health`) 0.0)
    (`self.OnDeath`)))

(fn `Die`
  (if (`|EnumEquality` (`self.Health Status`) "NewEnumerator0")
    (set `self.Health Status` "NewEnumerator1")))

(fn `Initialize Health Component`
  (set `self.Current Health` (`self.Max Health`)))

(fn `Take Damage`
  (params (Damage :type "Float (double-precision)"))
  (if (`|EnumEquality` (`self.Health Status`) "NewEnumerator0")
    (bind _output_get (set `self.Current Health` (`KismetMathLibrary.FClamp` (- (`self.Current Health`) Damage) 0.0 (`self.Max Health`))))
    (`KismetSystemLibrary.PrintString` (`KismetStringLibrary.Conv_DoubleToString` _output_get))
    (`self.OnHealthChanged`)))