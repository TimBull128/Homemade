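; BPC_Combat is an actor component that runs a bash attack with the weapon its owner holds.
; Attack checks that the item held in BPC_Inventory implements BPI_Weapons and no attack is running, then fires the AttackBegins dispatcher.
; The bound event plays the bash montage on the main and shadow meshes, clearing IsAttacking when it completes or is interrupted.
; The "Damage Window" montage notify enables and disables damage on the held weapon.
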(event `self.ReceiveBeginPlay`
  (add `self.Attack Begins` (delegate `Attack Begins_Event`)))

(event `Attack Begins_Event` :!signature `self.Attack Begins`
  (params (Mesh :type "SkeletalMeshComponent Object Reference") (`Shadow Mesh` :type "SkeletalMeshComponent Object Reference"))
  (bind _actor_held (`/Game/Blueprints/Functions/BPC_Inventory.Actor Held` (`Actor.GetComponentByClass` (`self.GetOwner`) "/Game/Blueprints/Functions/BPC_Inventory.BPC_Inventory_C")))
  (set `self.is Attacking?` true)
  (bind _notifyname (`|PlayMontage` Mesh "/Game/Characters/Imported/Player/Anims/Montage_Bash.Montage_Bash" 1.0 0.0 "None" false)
    (:`then`
      (`|PlayMontage` `Shadow Mesh` "/Game/Characters/Imported/Player/Anims/Montage_Bash.Montage_Bash" 1.0 0.0 "None" false))
    (:`OnCompleted`
      (set `self.is Attacking?` false :!label _label))
    (:`OnInterrupted`
      (goto _label))
    (:`OnNotifyBegin`
      (bind _returnvalue (== _notifyname "Damage Window"))
      (if _returnvalue
        (message `/Game/Blueprints/Functions/BPI_Weapons.Enable Damage` _actor_held)))
    (:`OnNotifyEnd`
      (if _returnvalue
        (message `/Game/Blueprints/Functions/BPI_Weapons.Disable Damage` _actor_held)))))

(fn `Attack`
  (params (Mesh :type "SkeletalMeshComponent Object Reference") (`Shadow Mesh` :type "SkeletalMeshComponent Object Reference"))
  (bind _actor_held (`/Game/Blueprints/Functions/BPC_Inventory.Actor Held` (`Actor.GetComponentByClass` (`self.GetOwner`) "/Game/Blueprints/Functions/BPC_Inventory.BPC_Inventory_C")))
  (`/Engine/EditorBlueprintResources/StandardMacros.IsValid` _actor_held
    (:`Is Valid`
      (if (and (`KismetSystemLibrary.DoesImplementInterface` _actor_held "/Game/Blueprints/Functions/BPI_Weapons.BPI_Weapons_C") (not (`self.is Attacking?`)))
        (`self.Attack Begins` Mesh `Shadow Mesh`)))))