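; Blueprint function library that saves, loads and creates the player's save game in a single fixed slot.
; Save writes a given save object to the slot, and Load reads it back as BP_Save if the slot exists.
; New Game creates a BP_Save with the player name and writes it immediately.
; Load and New Game both hand the resulting save object to the player actor's SaveFile variable.
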(fn `Load Game`
  (locals (`Save Game` :type "SaveGame Object Reference"))
  (bind _returnvalue (`GameplayStatics.DoesSaveGameExist` "SaveFile"))
  (if _returnvalue
    (bind _returnvalue_2 (`GameplayStatics.LoadGameFromSlot` "SaveFile"))
    (set `local.Save Game` _returnvalue_2)
    (bind _player_actor (`/Game/Blueprints/Functions/BPF_Casts.Get Player Actor` null))
    (`/Engine/EditorBlueprintResources/StandardMacros.IsValid` _player_actor
      (:`Is Valid`
        (bind _asbp_save (cast `/Game/Blueprints/Functions/BP_Save` (`local.Save Game`)))
        (set `/Game/FirstPerson/Blueprints/BP_FirstPersonCharacter.SaveFile` _asbp_save _player_actor)))))

(fn `New Game`
  (params (PlayerName :type String))
  (locals (Savefile :type "/Game/Blueprints/Functions/BP_Save Object Reference"))
  (bind _returnvalue (`GameplayStatics.CreateSaveGameObject` "/Game/Blueprints/Functions/BP_Save.BP_Save_C"))
  (bind _output_get (set `local.Savefile` _returnvalue))
  (set `/Game/Blueprints/Functions/BP_Save.PlayerName` PlayerName _output_get)
  (bind _returnvalue_2 (`GameplayStatics.SaveGameToSlot` (`local.Savefile`) "SaveFile"))
  (if _returnvalue_2
    (bind _player_actor (`/Game/Blueprints/Functions/BPF_Casts.Get Player Actor` null))
    (`/Engine/EditorBlueprintResources/StandardMacros.IsValid` _player_actor
      (:`Is Valid`
        (set `/Game/FirstPerson/Blueprints/BP_FirstPersonCharacter.SaveFile` (`local.Savefile`) _player_actor)))))

(fn `Save game`
  (params (`Save Game` :type "/Game/Blueprints/Functions/BP_Save Object Reference"))
  (`GameplayStatics.SaveGameToSlot` `Save Game` "SaveFile"))