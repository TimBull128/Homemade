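; Inventory component for a Character owner that tracks money and stores actors in separate Enemy, Weapon and Tool lists, each with its own index.
; Adding or cycling items broadcasts OnActorChanged, which hides the previous actor and attaches the new one to the MainHand socket, except Tool cycling, which calls an empty SetActorHeld.
; Removing the held actor spawns a replacement of its class, copies its details through message calls, then destroys the original.
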(event `self.ReceiveBeginPlay`
  (`|ExecutionSequence`
    (:`then_0`
      (bind _ascharacter (cast `Character` (`self.GetOwner`)))
      (set `self.Owner` _ascharacter))
    (:`then_1`
      (add `self.On Actor Changed` (delegate `On Actor Changed_Event`)))))

(event `On Actor Changed_Event`
  (params (`Actor Details` :type "/Game/Blueprints/Functions/Inventory/S_InventoryAssets Structure"))
  (bind _output (`|GetArrayItem` `Actor Details_Actors_5_8C4CCAFF425DF7AD96388EBCA6A19ADB` `Actor Details_Index_7_7851C67547B7B657D7148DA25AA02D3A`))
  (if (and (>= `Actor Details_Index_7_7851C67547B7B657D7148DA25AA02D3A` 0) (`KismetSystemLibrary.IsValid` _output))
    (bind _actor_held (`self.Actor Held`)
      (:`then`
        (`Actor.K2_DetachFromActor` _actor_held "KeepWorld" "KeepWorld" "KeepWorld")
        (`Actor.SetActorHiddenInGame` _actor_held true)
        (message `/Game/Blueprints/Functions/BPI_Interact.Set Object Collision` _actor_held "NoCollision"))
      (:`else`
        _))
    (bind _output_get (set `self.Actor Held` _output))
    (`Actor.SetActorHiddenInGame` _output_get false)
    (`Actor.K2_AttachToComponent` (`self.Actor Held`) (`Character.Mesh` (`self.Owner`)) (`self.Main Hand`) "SnapToTarget" "SnapToTarget" "KeepWorld" false)))

(fn `Add Money`
  (params (`Add Money` :type Integer))
  (set `self.Money` (+ `Add Money` (`self.Money`))))

(fn `Add New Inventory item`
  (params (`New Actor` :type "Actor Object Reference"))
  (locals (`Target actor` :type "Actor Object Reference"))
  (bind _enemies (`self.Enemies`))
  (bind _tools (`self.Tools`))
  (bind _weapons (`self.Weapons`))
  (bind _target_actor (`local.Target actor`))
  (`/Engine/EditorBlueprintResources/StandardMacros.IsValid` `New Actor`
    (:`Is Valid`
      (bind _output_get (set `local.Target actor` `New Actor`))
      (bind _actor_details (message `/Game/Blueprints/Functions/BPI_Interact.Get Actor Details` _output_get))
      (bind _output_get_2 (set `self.Inventory Type` (`.InventoryType_20_7964C2304E97BEB78DCB259AD7C0D2BE` (break `/Game/Blueprints/Functions/Inventory/S_ActorDetails` _actor_details))))
      (switch `/Game/Blueprints/Functions/Inventory/E_InventoryType` _output_get_2
        (:`NewEnumerator0`
          (`Actor.SetActorEnableCollision` _target_actor false)
          (bind _returnvalue (`KismetArrayLibrary.Array_AddUnique` (`.Actors_5_8C4CCAFF425DF7AD96388EBCA6A19ADB` (break `/Game/Blueprints/Functions/Inventory/S_InventoryAssets` _enemies)) (`local.Target actor`)))
          (bind _structout (setmembers `/Game/Blueprints/Functions/Inventory/S_InventoryAssets` :`StructRef` _enemies :`Index` _returnvalue))
          (`self.On Actor Changed` _structout))
        (:`NewEnumerator4`
          (message `/Game/Blueprints/Functions/BPI_Interact.Set Object Collision` _target_actor "NoCollision")
          (bind _returnvalue_2 (`KismetArrayLibrary.Array_AddUnique` (`.Actors_5_8C4CCAFF425DF7AD96388EBCA6A19ADB` (break `/Game/Blueprints/Functions/Inventory/S_InventoryAssets` _weapons)) (`local.Target actor`)))
          (bind _structout_2 (setmembers `/Game/Blueprints/Functions/Inventory/S_InventoryAssets` :`StructRef` _weapons :`Index` _returnvalue_2))
          (`self.On Actor Changed` _structout_2))
        (:`NewEnumerator5`
          (`Actor.SetActorEnableCollision` _target_actor false)
          (bind _returnvalue_3 (`KismetArrayLibrary.Array_AddUnique` (`.Actors_5_8C4CCAFF425DF7AD96388EBCA6A19ADB` (break `/Game/Blueprints/Functions/Inventory/S_InventoryAssets` _tools)) (`local.Target actor`)))
          (bind _structout_3 (setmembers `/Game/Blueprints/Functions/Inventory/S_InventoryAssets` :`StructRef` _tools :`Index` _returnvalue_3))
          (`self.On Actor Changed` _structout_3))))))

(fn `Get Current Actor Held`
  (returns (`Actor Held` :type "Actor Object Reference"))
  (return (`self.Actor Held`)))

(fn `Get Money`
  (returns (Money :type Integer))
  (return (`self.Money`)))

(fn `New IDX`
  (params (InputPin :type Integer) (S_InventoryAssets :type "/Game/Blueprints/Functions/Inventory/S_InventoryAssets Structure (by ref)"))
  (returns (ReturnValue :type Integer))
  (locals (ArrLen :type Integer :default 0))
  (bind (_actors _index) (break `/Game/Blueprints/Functions/Inventory/S_InventoryAssets` S_InventoryAssets))
  (bind _output_get (set `local.ArrLen` (`KismetArrayLibrary.Array_Length` _actors)))
  (if (== _output_get 0)
    (return -1)
    (else
      (return (`KismetMathLibrary.Clamp` (+ InputPin _index) 0 (- _output_get 1))))))

(fn `Remove Actor Held`
  (params (SpawnTransform :type "Transform Structure"))
  (returns (ReturnValue :type "Actor Object Reference"))
  (bind _actor_held (`self.Actor Held`))
  (`Actor.K2_DetachFromActor` _actor_held "KeepWorld" "KeepWorld" "KeepWorld")
  (bind _returnvalue (`|SpawnActorFromClass` (`GameplayStatics.GetObjectClass` _actor_held) SpawnTransform "Undefined" "MultiplyWithRoot" null null))
  (switch `/Game/Blueprints/Functions/Inventory/E_InventoryType` (`self.Inventory Type`)
    (:`NewEnumerator0`
      (`KismetArrayLibrary.Array_RemoveItem` (`.Actors_5_8C4CCAFF425DF7AD96388EBCA6A19ADB` (break `/Game/Blueprints/Functions/Inventory/S_InventoryAssets` (`self.Enemies`)))))
    (:`NewEnumerator4`
      (`KismetArrayLibrary.Array_RemoveItem` (`.Actors_5_8C4CCAFF425DF7AD96388EBCA6A19ADB` (break `/Game/Blueprints/Functions/Inventory/S_InventoryAssets` (`self.Weapons`)))))
    (:`NewEnumerator5`
      (`KismetArrayLibrary.Array_RemoveItem` (`.Actors_5_8C4CCAFF425DF7AD96388EBCA6A19ADB` (break `/Game/Blueprints/Functions/Inventory/S_InventoryAssets` (`self.Tools`))))))
  (bind _actor_details (message `/Game/Blueprints/Functions/BPI_Interact.Get Actor Details` _actor_held))
  (message `/Game/Blueprints/Functions/BPI_Interact.Set Actor Details` _returnvalue _actor_details)
  (`Actor.K2_DestroyActor` _actor_held)
  (return _returnvalue))

(fn `Set Actor Held`
  (params (Inventory :type "/Game/Blueprints/Functions/Inventory/S_InventoryAssets Structure")))

(fn `Update Actor Held`
  (params (`Index Update` :type Integer))
  (locals (`Update IDX` :type Integer))
  (set `local.Update IDX` `Index Update`)
  (switch `/Game/Blueprints/Functions/Inventory/E_InventoryType` (`self.Inventory Type`)
    (:`NewEnumerator0`
      (bind _returnvalue (`self.New IDX` (`local.Update IDX`) (`self.Enemies`)))
      (bind _structout (setmembers `/Game/Blueprints/Functions/Inventory/S_InventoryAssets` :`StructRef` (`self.Enemies`) :`Index` _returnvalue))
      (`self.On Actor Changed` _structout))
    (:`NewEnumerator4`
      (bind _returnvalue_2 (`self.New IDX` (`local.Update IDX`) (`self.Weapons`)))
      (bind _structout_2 (setmembers `/Game/Blueprints/Functions/Inventory/S_InventoryAssets` :`StructRef` (`self.Weapons`) :`Index` _returnvalue_2))
      (`self.On Actor Changed` _structout_2))
    (:`NewEnumerator5`
      (bind _returnvalue_3 (`self.New IDX` (`local.Update IDX`) (`self.Tools`)))
      (bind _structout_3 (setmembers `/Game/Blueprints/Functions/Inventory/S_InventoryAssets` :`StructRef` (`self.Tools`) :`Index` _returnvalue_3))
      (`self.Set Actor Held` _structout_3))))