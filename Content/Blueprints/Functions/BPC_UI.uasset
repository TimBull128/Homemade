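; BPC_UI is a component that holds a player's main UI and current interaction state, with prompt types for investigate, pickup, plant and harvest.
; SetUpUIParams stores the player controller, creates the UI_Main widget for it and adds it to the viewport.
; A stored InteractType has a getter and setter, and GetInteractText maps it to prompt text, with Investigate marked unimplemented.
; SwitchUI only adds the target widget to the viewport, without removing the current one.
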(fn `Get Interact Text`
  (returns (ReturnValue :type Text))
  (switch `/Game/Blueprints/Functions/E_InteractType` (`self.Interact Type`)
    (:`NewEnumerator0`
      (return ""))
    (:`NewEnumerator1`
      (return "Investigate (Not Implemented)"))
    (:`NewEnumerator2`
      (return "Pickup"))
    (:`NewEnumerator3`
      (return "Plant"))
    (:`NewEnumerator4`
      (return "Harvest"))))

(fn `Get Interact Type`
  (returns (`Interact Type` :type "/Game/Blueprints/Functions/E_InteractType Enum"))
  (return (`self.Interact Type`)))

(fn `Set Interact Type`
  (params (`Interact Type` :type "/Game/Blueprints/Functions/E_InteractType Enum" :default "NewEnumerator0"))
  (set `self.Interact Type` `Interact Type`))

(fn `Set Up UI Params`
  (params (`Player Controller` :type "PlayerController Object Reference"))
  (bind _output_get (set `self.Owning Player Controller` `Player Controller`))
  (bind _returnvalue (`|CreateWidget` "/Game/UI/Screens/UI_Main.UI_Main_C" _output_get))
  (bind _output_get_2 (set `self.Main UI` _returnvalue))
  (`UserWidget.AddToViewport` _output_get_2 0))

(fn `Switch UI`
  (params (Target :type "UserWidget Object Reference"))
  (`UserWidget.AddToViewport` Target 0))