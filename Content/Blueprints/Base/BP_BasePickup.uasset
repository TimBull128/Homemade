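; BP_BasePickup is a base pickup actor that puts itself into the interacting actor's inventory.
; It reports a fixed interact type through GetInteractType.
; On Interact, it confirms that the caller's BPC_UI component holds that same interact type, then passes itself to the caller's BPC_Inventory through AddNewInventoryItem.
; Validity checks guard each component lookup, and the pickup does not destroy or hide itself here.
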(event `/Game/Blueprints/Functions/BPI_Interact.Interact`
  (params (`Calling Actor` :type "Character Object Reference"))
  (bind _returnvalue (`self.GetComponentByClass` `Calling Actor` "/Game/Blueprints/Functions/BPC_UI.BPC_UI_C"))
  (bind _returnvalue_2 (`self.GetComponentByClass` `Calling Actor` "/Game/Blueprints/Functions/Inventory/BPC_Inventory.BPC_Inventory_C"))
  (`/Engine/EditorBlueprintResources/StandardMacros.IsValid` `Calling Actor`
    (:`Is Valid`
      (`/Engine/EditorBlueprintResources/StandardMacros.IsValid` _returnvalue
        (:`Is Valid`
          (if (`|EnumEquality` (`/Game/Blueprints/Functions/BPC_UI.Get Interact Type` _returnvalue) "NewEnumerator2")
            (`/Engine/EditorBlueprintResources/StandardMacros.IsValid` _returnvalue_2
              (:`Is Valid`
                (`/Game/Blueprints/Functions/Inventory/BPC_Inventory.Add New Inventory item` _returnvalue_2 self)))))))))

(fn `Get Interact Type`
  (params (`Calling Actor` :type "Character Object Reference"))
  (returns (NewParam :type "/Game/Blueprints/Functions/E_InteractType Enum"))
  (return "NewEnumerator2"))

(fn `UserConstructionScript`)