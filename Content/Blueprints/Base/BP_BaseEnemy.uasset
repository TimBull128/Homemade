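; Base enemy actor that takes combat hits and reports an interaction type based on its health state.
; The construction script reads its data table row to set the static mesh and max health.
; Received attacks arrive through a combat component binding, which processes the hit and passes the result to the health component as damage.
; GetInteractType maps the health component's status to an interact type for the calling actor.
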(event `self.ReceiveBeginPlay`
  (`parent.ReceiveBeginPlay`)
  (`/Game/Blueprints/Functions/BPC_Health.Initialize Health Component` (`self.BPC_Health`))
  (add `/Game/Blueprints/Functions/BPC_Combat.Attack Recieved` (`self.BPC_Combat`) (delegate `Event Attack Recieved`)))

(event `Event Attack Recieved`
  (params (Target :type "Actor Object Reference") (Weapon :type "Actor Object Reference"))
  (bind _damage (`/Game/Blueprints/Functions/BPC_Combat.Process Incoming Hit` (`self.BPC_Combat`) Target Weapon))
  (`/Game/Blueprints/Functions/BPC_Health.Take Damage` (`self.BPC_Health`) _damage))

(fn `Get Interact Type`
  (params (`Calling Actor` :type "Character Object Reference"))
  (returns (NewParam :type "/Game/Blueprints/Functions/E_InteractType Enum"))
  (if (`|EnumEquality` (`/Game/Blueprints/Functions/BPC_Health.Health Status` (`self.BPC_Health`)) "NewEnumerator1")
    (return "NewEnumerator2")
    (elif (`|EnumEquality` (`/Game/Blueprints/Functions/BPC_Health.Health Status` (`self.BPC_Health`)) "NewEnumerator2")
      (return "NewEnumerator1")
      (else
        (return "NewEnumerator0")))))

(fn `UserConstructionScript`
  (bind (_datatable _rowname) (break `DataTableRowHandle` (`.ActorDetails_44_B50C7B50436276A2E83B66962C7791D8` (break `/Game/Blueprints/Functions/Inventory/S_ActorDetails` (`self.Actor Details`)))))
  (`parent.UserConstructionScript`)
  (bind _returnvalue (`|GetDataTableRow` _datatable _rowname)
    (:`then`
      (bind (_moneyadded _burytime _mesh _maxhealth) (break `/Game/Blueprints/Functions/Inventory/Tables/S_EnemyStat` _returnvalue))
      (`StaticMeshComponent.SetStaticMesh` (`self.Object`) _mesh)
      (set `/Game/Blueprints/Functions/BPC_Health.Max Health` (`KismetMathLibrary.Conv_IntToDouble` _maxhealth) (`self.BPC_Health`)))))