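; Base farm plot where a player buries a held enemy and later harvests it for gold.
; Interact plants or harvests via the player's BPC_Inventory, reading bury time and reward from the planted actor.
; An OnStatusChange dispatcher drives Open, Growing and Harvestable visuals; a looping one-second timer counts down, then the buried actor is destroyed.
; Tick smoothly turns the countdown label toward the planter's camera.
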(event `self.ReceiveBeginPlay`
  (`parent.ReceiveBeginPlay`)
  (`SceneComponent.SetHiddenInGame` (`self.Time pivot`) true true)
  (`SceneComponent.SetVisibility` (`self.CollectionObject`) false false)
  (add `self.On Status Change` (delegate `Event On Status Change`)))

(event `Event On Status Change`
  (switch `/Game/Blueprints/Functions/E_Planted_Status` (`self.Plant Status`)
    (:`NewEnumerator0`
      (`self.Set Ready`))
    (:`NewEnumerator1`
      (`self.Set Harvestable`))
    (:`NewEnumerator2`
      (`self.Set Growing`))))

(event `/Game/Blueprints/Functions/BPI_Interact.Interact`
  (params (`Calling Actor` :type "Character Object Reference"))
  (`/Engine/EditorBlueprintResources/StandardMacros.IsValid` `Calling Actor`
    (:`Is Valid`
      (bind _output_get (set `self.Calling Actor` `Calling Actor`))
      (switch `/Game/Blueprints/Functions/E_Planted_Status` (`self.Plant Status`)
        (:`NewEnumerator0`
          (bind _returnvalue (`self.GetComponentByClass` _output_get "/Game/Blueprints/Functions/BPC_Inventory.BPC_Inventory_C"))
          (`/Engine/EditorBlueprintResources/StandardMacros.IsValid` _returnvalue
            (:`Is Valid`
              (bind _actor_held (`/Game/Blueprints/Functions/BPC_Inventory.Actor Held` _returnvalue)
                (:`then`
                  (if (`KismetSystemLibrary.DoesImplementInterface` _actor_held "/Game/Blueprints/Functions/BPI_Enemy.BPI_Enemy_C")
                    (`self.Plant Actor`)))
                (:`else`)))))
        (:`NewEnumerator1`
          (`self.Harvest Actor`))))))

(event `self.ReceiveTick`
  (params (DeltaSeconds :type "Float (single-precision)"))
  (bind _following_actor (`self.Following Actor`)
    (:`then`
      (bind _returnvalue (`self.GetComponentByClass` _following_actor "/Script/Engine.CameraComponent"))
      (`/Engine/EditorBlueprintResources/StandardMacros.IsValid` _returnvalue
        (:`Is Valid`
          (`SceneComponent.K2_SetWorldRotation` (`self.Time pivot`) (`KismetMathLibrary.RInterpTo` (`SceneComponent.K2_GetComponentRotation` (`self.Time pivot`)) (`KismetMathLibrary.FindLookAtRotation` (`SceneComponent.K2_GetComponentLocation` (`self.Time pivot`)) (`SceneComponent.K2_GetComponentLocation` _returnvalue)) DeltaSeconds 3.0) false false))))
    (:`else`)))

(fn `Farm Timer Func`
  (bind _planted_counter (`self.Planted Counter`))
  (if (> _planted_counter 0)
    (`/Engine/EditorBlueprintResources/StandardMacros.DecrementInt` _planted_counter
      (:`  `
        (`TextRenderComponent.K2_SetText` (`self.Time`) (`KismetTextLibrary.Conv_StringToText` (`KismetStringLibrary.Concat_StrStr` (`KismetStringLibrary.Conv_IntToString` (`self.Planted Counter`)) "s")))))
    (else
      (set `self.Plant Status` "NewEnumerator1")
      (`self.On Status Change`))))

(fn `Get Interact Type`
  (params (`Calling Actor` :type "Character Object Reference"))
  (returns (NewParam :type "/Game/Blueprints/Functions/E_InteractType Enum"))
  (bind _returnvalue (`self.GetComponentByClass` `Calling Actor` "/Game/Blueprints/Functions/BPC_Inventory.BPC_Inventory_C"))
  (switch `/Game/Blueprints/Functions/E_Planted_Status` (`self.Plant Status`)
    (:`NewEnumerator0`
      (`/Engine/EditorBlueprintResources/StandardMacros.IsValid` `Calling Actor`
        (:`Is Valid`
          (`/Engine/EditorBlueprintResources/StandardMacros.IsValid` _returnvalue
            (:`Is Valid`
              (bind _actor_held (`/Game/Blueprints/Functions/BPC_Inventory.Actor Held` _returnvalue)
                (:`then`
                  (bind _actor_details (message `/Game/Blueprints/Functions/BPI_Interact.Get Actor Details` _actor_held))
                  (if (`|EnumEquality` (`.InventoryType_20_7964C2304E97BEB78DCB259AD7C0D2BE` (break `/Game/Blueprints/Functions/S_ActorDetails` _actor_details)) "NewEnumerator0")
                    (return "NewEnumerator3")
                    (else
                      _)))
                (:`else`
                  _)))
            (:`Is Not Valid`
              _)))
        (:`Is Not Valid`
          _)))
    (:`NewEnumerator1`
      (return "NewEnumerator4"))
    (:`NewEnumerator2`
      _))
  (return "NewEnumerator1"))

(fn `Get Planted Status`
  (returns (`Actor Planted?` :type "/Game/Blueprints/Functions/E_Planted_Status Enum"))
  (return (`self.Plant Status`)))

(fn `Harvest Actor`
  (bind _calling_actor (`self.Calling Actor`))
  (bind _returnvalue (`self.GetComponentByClass` _calling_actor "/Game/Blueprints/Functions/BPC_Inventory.BPC_Inventory_C"))
  (`/Engine/EditorBlueprintResources/StandardMacros.IsValid` _calling_actor
    (:`Is Valid`
      (`/Engine/EditorBlueprintResources/StandardMacros.IsValid` _returnvalue
        (:`Is Valid`
          (`/Game/Blueprints/Functions/BPC_Inventory.Add Money` _returnvalue (`self.Gold Awarded`))
          (set `self.Plant Status` "NewEnumerator0")
          (`self.On Status Change`))))))

(fn `Plant Actor`
  (bind _calling_actor (`self.Calling Actor`))
  (bind (_returnvalue_location _returnvalue_rotation) (`KismetMathLibrary.BreakTransform` (`SceneComponent.K2_GetComponentToWorld` (`self.Attachpoint`))))
  (bind _returnvalue (`self.GetComponentByClass` _calling_actor "/Game/Blueprints/Functions/BPC_Inventory.BPC_Inventory_C"))
  (set `self.Following Actor` _calling_actor)
  (`/Engine/EditorBlueprintResources/StandardMacros.IsValid` _returnvalue
    (:`Is Valid`
      (bind _returnvalue_2 (`/Game/Blueprints/Functions/BPC_Inventory.Detach Actor Held` _returnvalue (`KismetMathLibrary.MakeTransform` _returnvalue_location _returnvalue_rotation)))
      (bind _output_get (set `self.Actor Planted` _returnvalue_2))
      (bind _actor_details (message `/Game/Blueprints/Functions/BPI_Interact.Get Actor Details` _output_get))
      (bind (_name _icon _burytime _ispickupable_ _inventorytype _isplantable_ _goldawarded) (break `/Game/Blueprints/Functions/S_ActorDetails` _actor_details))
      (set `self.Planted Counter` _burytime)
      (set `self.Gold Awarded` _goldawarded)
      (set `self.Plant Status` "NewEnumerator2")
      (`self.On Status Change`))))

(fn `Set Growing`
  (`SceneComponent.SetHiddenInGame` (`self.Time pivot`) false true)
  (bind _output_get (set `self.Label Text` "Time to Complete"))
  (`TextRenderComponent.K2_SetText` (`self.Label`) _output_get)
  (`TextRenderComponent.K2_SetText` (`self.Time`) (`KismetTextLibrary.Conv_StringToText` (`KismetStringLibrary.Concat_StrStr` (`KismetStringLibrary.Conv_IntToString` (`self.Planted Counter`)) "s")))
  (bind _returnvalue (`KismetSystemLibrary.K2_SetTimer` null "Farm Timer Func" 1.0 true))
  (set `self.Farm Timer` _returnvalue)
  (set `self.Following Actor` (`self.Calling Actor`)))

(fn `Set Harvestable`
  (`KismetSystemLibrary.K2_ClearAndInvalidateTimerHandle` (`self.Farm Timer`))
  (`self.K2_DestroyActor` (`self.Actor Planted`))
  (set `self.Actor Planted` null)
  (`SceneComponent.SetVisibility` (`self.CollectionObject`) true false)
  (`PrimitiveComponent.SetCollisionEnabled` (`self.CollectionObject`) "QueryAndPhysics")
  (bind _output_get (set `self.Label Text` "Ready To Harvest!"))
  (`TextRenderComponent.K2_SetText` (`self.Label`) _output_get)
  (`SceneComponent.SetVisibility` (`self.Time`) false false))

(fn `Set Ready`
  (`PrimitiveComponent.SetCollisionEnabled` (`self.CollectionObject`) "NoCollision")
  (`SceneComponent.SetHiddenInGame` (`self.Time pivot`) true true)
  (`SceneComponent.SetHiddenInGame` (`self.CollectionObject`) true false)
  (set `self.Following Actor` null))

(fn `UserConstructionScript`
  (`parent.UserConstructionScript`))