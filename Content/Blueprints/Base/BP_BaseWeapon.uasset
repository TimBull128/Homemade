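; BP_BaseWeapon is a base weapon Blueprint that takes its mesh from a data table and reports hits from a collision component.
; The construction script looks up the WeaponID row and applies its static mesh.
; HitCollision overlaps fire the OnWeaponHit dispatcher with the other actor, while EnableDamage switches that collision between query-only and disabled.
; The Interact function is an empty stub.
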(event `self.Hit Collision.OnComponentBeginOverlap`
  (params (OverlappedComponent :type "PrimitiveComponent Object Reference") (OtherActor :type "Actor Object Reference") (OtherComp :type "PrimitiveComponent Object Reference") (OtherBodyIndex :type Integer) (bFromSweep :type Boolean) (SweepResult :type "HitResult Structure (by ref)"))
  (`self.OnWeaponHit` OtherActor))

(event `/Game/Blueprints/Functions/BPI_Weapons.Enable Damage`
  (params (`Enable Damage?` :type Boolean))
  (bind _hit_collision (`self.Hit Collision`))
  (if `Enable Damage?`
    (`PrimitiveComponent.SetCollisionEnabled` _hit_collision "QueryOnly")
    (else
      (`PrimitiveComponent.SetCollisionEnabled` _hit_collision "NoCollision"))))

(fn `Interact_0`)

(fn `UserConstructionScript`
  (bind (_datatable _rowname) (break `DataTableRowHandle` (`self.Weapon ID`)))
  (`parent.UserConstructionScript`)
  (bind _returnvalue (`|GetDataTableRow` _datatable _rowname)
    (:`then`
      (`StaticMeshComponent.SetStaticMesh` (`self.Object`) (`.CurrentMesh_25_395F785E4B2F98BB8D6815B44A99609B` (break `/Game/Blueprints/Functions/S_WeaponStat` _returnvalue))))))